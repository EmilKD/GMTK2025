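; BP_Tree is an environment prop that places a tree static mesh with per-instance variation.
; Its construction script picks a mesh from the Trees array, either at random or by TreeType.
; It then applies random rotation jitter around a 90-degree roll, plus a random scale offset on a slightly Z-stretched default scale.
; Unseeded randomness re-rolls whenever construction reruns, and the event graph holds no logic.
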(fn `UserConstructionScript`
  (bind _tree (`self.tree`))
  (bind _trees (`self.trees`))
  (bind _returnvalue (* (* (- (`KismetMathLibrary.RandomFloat`) 0.5) 2.0) (`self.rotationrand`)))
  (if (`self.random`)
    (`StaticMeshComponent.SetStaticMesh` _tree (`|GetArrayItem` _trees (`KismetMathLibrary.RandomInteger` (`KismetArrayLibrary.Array_Length` _trees))))
    (else
      (`StaticMeshComponent.SetStaticMesh` _tree (`|GetArrayItem` (`self.trees`) (`self.TreeType`)))))
  (`SceneComponent.K2_SetRelativeRotation` _tree (`KismetMathLibrary.MakeRotator` (+ _returnvalue 90.0) _returnvalue _returnvalue) false false)
  (`SceneComponent.SetRelativeScale3D` (`self.tree`) (+ (* (`KismetMathLibrary.MakeVector` 1.0 1.0 1.2) (`self.defaultscale`)) (* (* (- (`KismetMathLibrary.RandomFloat`) 0.5) 2.0) (`self.scalerand`)))))