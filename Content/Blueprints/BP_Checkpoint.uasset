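; BP_Checkpoint is a checkpoint actor that saves the player's spawn state when the player enters its trigger.
; On overlap with the player pawn, it writes its CheckpointType to SpawnState on the BP_PT_GameInstance save object and saves it to that instance's slot.
; It then disables actor tick, which leaves the overlap trigger active.
; The construction script labels the TextRender with the checkpoint type's name.
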(event `self.ReceiveBeginPlay`)

(event `self.Trigger.OnComponentBeginOverlap`
  (params (OverlappedComponent :type "PrimitiveComponent Object Reference") (OtherActor :type "Actor Object Reference") (OtherComp :type "PrimitiveComponent Object Reference") (OtherBodyIndex :type Integer) (bFromSweep :type Boolean) (SweepResult :type "HitResult Structure (by ref)"))
  (if (== OtherActor (`GameplayStatics.GetPlayerPawn` 0))
    (bind _asbp_pt_game_instance (cast `/Game/Blueprints/GameModes/BP_PT_GameInstance` (`GameplayStatics.GetGameInstance`)))
    (bind _thesavegame (`/Game/Blueprints/GameModes/BP_PT_GameInstance.TheSaveGame` _asbp_pt_game_instance))
    (set `/Game/Blueprints/GameModes/BPSG_Stats.SpawnState` (`self.CheckpointType`) _thesavegame)
    (`GameplayStatics.SaveGameToSlot` _thesavegame (`/Game/Blueprints/GameModes/BP_PT_GameInstance.SlotName` _asbp_pt_game_instance))
    (`self.SetActorTickEnabled` false)))

(fn `UserConstructionScript`
  (`TextRenderComponent.K2_SetText` (`self.TextRender`) (`KismetTextLibrary.Conv_StringToText` (`|GetEnumeratorNameAsString` (`self.CheckpointType`)))))