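; Game instance that owns the BPSG_Stats save and tracks the gameplay loop of hole fall, enemy wave and boss.
; On Init it loads the slot or creates a new save, prints the stored GamePlayState, advances it one step and saves, so each launch moves the loop forward.
; This is debug scaffolding: the boss outcome uses RandomInteger(1), which always returns 0, so it always ends in game over.
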(event `self.ReceiveInit`
  (`self.LoadFromSave`)
  ;[1 1 1] Just a debug presenation of the save game
  (switch `/Game/Blueprints/GameModes/E_LoopState` (`/Game/Blueprints/GameModes/BPSG_Stats.GamePlayState` (`self.TheSaveGame`))
    (:`NewEnumerator0`
      (`KismetSystemLibrary.PrintString` "Current Is Start \nYou should jump into hole" true true (struct :`R` 1.0 :`G` 0.065753 :`A` 1.0) 10.0)
      (set `/Game/Blueprints/GameModes/BPSG_Stats.GamePlayState` "NewEnumerator1" (`self.TheSaveGame`)))
    (:`NewEnumerator1`
      (`KismetSystemLibrary.PrintString` "Current Is Wake up and jump \nYou are now falling" true true (struct :`R` 1.0 :`G` 0.033409 :`A` 1.0) 10.0)
      (set `/Game/Blueprints/GameModes/BPSG_Stats.GamePlayState` "NewEnumerator2" (`self.TheSaveGame`)))
    (:`NewEnumerator2`
      (`KismetSystemLibrary.PrintString` "Current Is AfterFall \nYou should fight for your life" true true (struct :`R` 1.0 :`A` 1.0) 10.0)
      (set `/Game/Blueprints/GameModes/BPSG_Stats.GamePlayState` "NewEnumerator3" (`self.TheSaveGame`)))
    (:`NewEnumerator3`
      (`KismetSystemLibrary.PrintString` "Current Is Handling wave \nIf you die by these enemies it would be a bummer. I you handled it well next up is BOSSSSSS" true true (struct :`R` 1.0 :`G` 0.095177 :`A` 1.0) 10.0)
      (set `/Game/Blueprints/GameModes/BPSG_Stats.GamePlayState` "NewEnumerator4" (`self.TheSaveGame`)))
    (:`NewEnumerator4`
      (`KismetSystemLibrary.PrintString` "Current Is Boss \nIf you kill the boss keep your resources and boss will throw you in the next hole, but if boss kills you. you will wake up to the jump in hole" true true (struct :`R` 1.0 :`B` 0.006452 :`A` 1.0) 10.0)
      (if (> (`KismetMathLibrary.RandomInteger` 1) 0)
        (set `/Game/Blueprints/GameModes/BPSG_Stats.GamePlayState` "NewEnumerator6" (`self.TheSaveGame`))
        (else
          (set `/Game/Blueprints/GameModes/BPSG_Stats.GamePlayState` "NewEnumerator7" (`self.TheSaveGame`)))))
    (:`NewEnumerator6`
      (`KismetSystemLibrary.PrintString` "Current boss killed \nYou go for the next fall" true true (struct :`R` 1.0 :`B` 0.067408 :`A` 1.0) 10.0)
      (set `/Game/Blueprints/GameModes/BPSG_Stats.GamePlayState` "NewEnumerator2" (`self.TheSaveGame`)))
    (:`NewEnumerator7`
      (`KismetSystemLibrary.PrintString` "Current you are killed by boss \ngo for the wake up call." true true (struct :`R` 1.0 :`B` 0.051723 :`A` 1.0) 10.0)
      (set `/Game/Blueprints/GameModes/BPSG_Stats.GamePlayState` "NewEnumerator1" (`self.TheSaveGame`))))
  (`self.SaveTheSaveGame`))

(fn `LoadFromSave`
  (bind _returnvalue (`GameplayStatics.DoesSaveGameExist` (`self.SlotName`)))
  (if _returnvalue
    (bind _returnvalue_2 (`GameplayStatics.LoadGameFromSlot` (`self.SlotName`)))
    (bind _asbpsg_stats (cast `/Game/Blueprints/GameModes/BPSG_Stats` _returnvalue_2))
    (set `self.TheSaveGame` _asbpsg_stats)
    (else
      (bind _returnvalue_3 (`GameplayStatics.CreateSaveGameObject` "/Game/Blueprints/GameModes/BPSG_Stats.BPSG_Stats_C"))
      (`GameplayStatics.SaveGameToSlot` _returnvalue_3 (`self.SlotName`))
      (set `self.TheSaveGame` _returnvalue_3))))

(fn `SaveTheSaveGame`
  (`GameplayStatics.SaveGameToSlot` (`self.TheSaveGame`) (`self.SlotName`)))