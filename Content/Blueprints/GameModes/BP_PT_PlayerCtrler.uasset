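; Player controller that sets up hero input and offers debug checkpoint hotkeys.
; On BeginPlay it adds the IMC_Hero Enhanced Input mapping context.
; Debug keys F7 and F6 call BP_PlayerState to save the player transform and to debug-spawn the player at a location.
; An unconnected camera optimization draft, attaching the camera manager to a spring arm on BP_BigFatHero, never runs.
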(event EventBeginPlay
  (Utilities|FlowControl|Sequence
    (:then_1
      (Input|AddMappingContext (PlayerController|LocalPlayerSubsystems|GetEnhancedInputLocalPlayerSubsystem self) "/Game/Inputs/IMC_Hero.IMC_Hero" 0 "(bIgnoreAllPressedKeysUntilRelease=True,bForceImmediately=False,bNotifyUserSettings=False)"))))

(event EventTick
  (params (DeltaSeconds :type Float%20%28single-precision%29)))

(event Input|KeyboardEvents|DebugKeyF7
  (params (Key :type Key%20Structure :default "None") (ActionValue :type Input%20Action%20Value%20Structure))
  ;[1 1 1] Checkpoint
  (:Pressed
    (bind _asbp_player_state (Utilities|Casting|CastToBP_PlayerState (Game|GetPlayerState 0)))
    (Default|SavePlayerTransform _asbp_player_state)))

(event Input|KeyboardEvents|DebugKeyF6
  (params (Key :type Key%20Structure :default "None") (ActionValue :type Input%20Action%20Value%20Structure))
  ;[1 1 1] Checkpoint
  (:Pressed
    (bind _asbp_player_state (Utilities|Casting|CastToBP_PlayerState (Game|GetPlayerState 0)))
    (Default|DebugSpawnPlayeratLocation _asbp_player_state)))

(fn ConstructionScript)