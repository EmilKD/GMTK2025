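; Player state that links the first local player to the save game for storing and restoring their location.
; On BeginPlay it caches the game mode, slot name and save object from the game instance, then runs a debug seed increment, log and save.
; SavePlayerTransform writes the pawn's transform and spawn state to the slot, and a debug function teleports the pawn back there.
; Each acts only when this is player 0's state; IsPlayerZero is an empty stub.
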(event `self.ReceiveBeginPlay`
  (bind _the_save_game (`self.The Save Game`))
  (bind _asbp_pt_game_instance (cast `/Game/Blueprints/GameModes/BP_PT_GameInstance` (`GameplayStatics.GetGameInstance`) :!pure true))
  (bind _currentseed (`/Game/Blueprints/GameModes/BPSG_Stats.CurrentSeed` _the_save_game))
  (if (== (`Pawn.PlayerState` (`GameplayStatics.GetPlayerPawn` 0)) self)
    (bind _asgm_game_mode_base (cast `/Game/Blueprints/GameModes/GM_GameModeBase` (`GameplayStatics.GetGameMode`)))
    (set `self.As GM Game Mode` _asgm_game_mode_base)
    (set `self.Slot Name` (`/Game/Blueprints/GameModes/BP_PT_GameInstance.SlotName` _asbp_pt_game_instance))
    (set `self.The Save Game` (`/Game/Blueprints/GameModes/BP_PT_GameInstance.TheSaveGame` _asbp_pt_game_instance))
    (bind _asbp_player_state (cast `/Game/Blueprints/GameModes/BP_PlayerState` (`Pawn.PlayerState` (`GameplayStatics.GetPlayerPawn` 0))))
    (set `self.Current Player State` _asbp_player_state)
    ;[0 1 1] Debug use of save game
    (bind _result (`/Engine/EditorBlueprintResources/StandardMacros.IncrementInt` _currentseed)
      (:`  `
        (`KismetArrayLibrary.Array_Add` (`/Game/Blueprints/GameModes/BPSG_Stats.PreviousSeeds` _the_save_game) _result)
        (`GameplayStatics.SaveGameToSlot` (`self.The Save Game`) (`self.Slot Name`))
        (`KismetSystemLibrary.PrintString` (`KismetStringLibrary.Conv_IntToString` _currentseed))))))

(fn `Debug Spawn Player At Location`
  (if (== (`Pawn.PlayerState` (`GameplayStatics.GetPlayerPawn` 0)) self)
    (`self.K2_SetActorTransform` (`GameplayStatics.GetPlayerPawn` 0) (`/Game/Blueprints/GameModes/BPSG_Stats.LastLocation` (`self.The Save Game`)) false true)))

(fn `IsPlayerZero`)

(fn `SavePlayerTransform`
  (if (== (`Pawn.PlayerState` (`GameplayStatics.GetPlayerPawn` 0)) self)
    (set `/Game/Blueprints/GameModes/BPSG_Stats.LastLocation` (`self.GetTransform` (`GameplayStatics.GetPlayerPawn` 0)) (`self.The Save Game`))
    (set `/Game/Blueprints/GameModes/BPSG_Stats.SpawnState` "NewEnumerator2" (`self.The Save Game`))
    (`GameplayStatics.SaveGameToSlot` (`self.The Save Game`) (`self.Slot Name`))))

(fn `UserConstructionScript`)