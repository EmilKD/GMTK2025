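; BP_Hero is a player character Blueprint with Enhanced Input actions for jumping, moving along a single axis and shooting.
; Movement scales the actor's forward vector by the input value and snaps the mesh yaw to face the travel direction.
; Shooting spawns BP_Bullet at BulletSpawnPoint and sets its sphere's physics velocity along the mesh's forward vector.
; Leftover mouse-to-screen direction nodes are unconnected and never run.
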(event `self.ReceiveTick`
  (params (DeltaSeconds :type "Float (single-precision)")))

(event `EnhancedInput|/Game/Inputs/IA_Jump`
  (params (ActionValue :type "Float (double-precision)") (ElapsedSeconds :type "Float (double-precision)") (TriggeredSeconds :type "Float (double-precision)") (InputAction :type "InputAction Object Reference" :default "/Game/Inputs/IA_Jump.IA_Jump"))
  (:`Triggered`
    (`self.Jump`)))

(event `EnhancedInput|/Game/Inputs/IA_Move`
  (params (ActionValue :type "Float (double-precision)") (ElapsedSeconds :type "Float (double-precision)") (TriggeredSeconds :type "Float (double-precision)") (InputAction :type "InputAction Object Reference" :default "/Game/Inputs/IA_Move.IA_Move"))
  (bind _scene (`self.Scene`))
  (:`Triggered`
    (`self.AddMovementInput` (* ActionValue (`self.GetActorForwardVector`)))
    (if (> ActionValue 0.0)
      (`SceneComponent.K2_SetWorldRotation` _scene (`KismetMathLibrary.MakeRotator` 0.0) false false)
      (`SceneComponent.K2_SetWorldRotation` (`self.Mesh`) (`KismetMathLibrary.MakeRotator` 0.0) false false)
      (else
        (`SceneComponent.K2_SetWorldRotation` _scene (`KismetMathLibrary.MakeRotator` 0.0 0.0 180.0) false false)
        (`SceneComponent.K2_SetWorldRotation` (`self.Mesh`) (`KismetMathLibrary.MakeRotator` 0.0 0.0 180.0) false false)))))

(event `EnhancedInput|/Game/Inputs/IA_Shoot`
  (params (ActionValue :type "Float (double-precision)") (ElapsedSeconds :type "Float (double-precision)") (TriggeredSeconds :type "Float (double-precision)") (InputAction :type "InputAction Object Reference" :default "/Game/Inputs/IA_Shoot.IA_Shoot"))
  (:`Triggered`
    (bind _returnvalue (`|SpawnActorFromClass` "/Game/Blueprints/BP_Bullet.BP_Bullet_C" (`SceneComponent.K2_GetComponentToWorld` (`self.BulletSpawnPoint`)) "Undefined" "MultiplyWithRoot" null null))
    (`PrimitiveComponent.SetPhysicsLinearVelocity` (`/Game/Blueprints/BP_Bullet.Sphere` _returnvalue) (* (`SceneComponent.GetForwardVector` (`self.Mesh`)) 5000.0) false "None")))

(fn `UserConstructionScript`
  (`parent.UserConstructionScript`))