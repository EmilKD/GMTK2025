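; Flipbook-based boss character, configured from a data asset, that wakes when the player overlaps its BossInit trigger.
; A single looping timer handle switches states: positioning tracks the player, attacking runs in range, and defending raises shields whenever any BP_Bullet exists.
; Combo1 chains three flipbook-timed sphere-trace hits that damage and launch the player, aborting if hurt.
; Shields block damage; Tick triggers faster rage mode at low HP, then death below zero.
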(event `self.ReceiveBeginPlay`
  (bind _sprite (`self.Sprite`))
  ;[1 1 1] Should RISE at the presence of the palyer
  (`self.FindFlipbookBySpritAnimState` "Fall")
  (`self.Face Toward Player`)
  (`KismetSystemLibrary.K2_SetTimerDelegate` (delegate `RISEEE`) (/ (`PaperFlipbookComponent.GetFlipbookLength` _sprite) (`PaperFlipbookComponent.GetPlayRate` _sprite))))

(event `RISEEE`
  ;[1 1 1] Should RISE at the presence of the palyer
  (`PaperFlipbookComponent.Stop` (`self.Sprite`)))

(event `self.TakeDamage`
  (params (Damage :type "Float (single-precision)") (DamageCauser :type "Actor Object Reference"))
  (if (not (`self.Shields up`))
    (`parent.TakeDamage` Damage DamageCauser)
    (`self.InterruptCombo`)
    (set `self.BossHP` (- (`self.BossHP`) Damage))))

(event `self.ReceiveTick`
  (params (DeltaSeconds :type "Float (single-precision)"))
  (`|ExecutionSequence`
    (:`then_0`
      (if (< (`self.BossHP`) (`self.RageThreshold`))
        (`self.RageMode`)
        (if (< (`self.BossHP`) 0.0)
          (set `self.IsDead` true)
          (`KismetSystemLibrary.K2_ClearAndInvalidateTimerHandle` (`self.TH_Tick`))
          (`PaperFlipbookComponent.SetPlayRate` (`self.Sprite`) 0.5)
          (`self.DeadScene`))))
    (:`then_1`
      (`SceneComponent.K2_SetWorldRotation` (`self.HPWidget`) (struct :`Yaw` 90.0) false false))))

(event `DeadScene`
  (bind _sprite (`self.Sprite`))
  (`self.SetActorTickEnabled` false)
  (`self.FindFlipbookBySpritAnimState` "Death")
  (`KismetSystemLibrary.Delay` (/ (`PaperFlipbookComponent.GetFlipbookLength` _sprite) (`PaperFlipbookComponent.GetPlayRate` _sprite) 4.0))
  (`PaperFlipbookComponent.Stop` (`self.Sprite`)))

(event `self.Boss init.OnComponentBeginOverlap`
  (params (OverlappedComponent :type "PrimitiveComponent Object Reference") (OtherActor :type "Actor Object Reference") (OtherComp :type "PrimitiveComponent Object Reference") (OtherBodyIndex :type Integer) (bFromSweep :type Boolean) (SweepResult :type "HitResult Structure (by ref)"))
  (if (== OtherActor (`GameplayStatics.GetPlayerPawn` 0))
    (`/Engine/EditorBlueprintResources/StandardMacros.DoOnce` false
      (:`Completed`
        (`PrimitiveComponent.SetCollisionEnabled` (`self.Boss init`) "NoCollision")
        (`KismetSystemLibrary.Delay` 1.0)
        (`self.GoForPositioning`)))))

(event `Combo1`
  (bind _sprite (`self.Sprite`))
  (bind _sprite_2 (`self.Sprite`))
  (bind _sprite_3 (`self.Sprite`))
  (`/Engine/EditorBlueprintResources/StandardMacros.DoOnce` false :!label _label
    (:`Completed`
      (set `self.IsAttacking` true)
      (`self.FindFlipbookBySpritAnimState` "Attack1")
      (`SceneComponent.K2_AddRelativeLocation` (`self.Sprite`) (-100.0 0.0 0.0) false true)
      (`self.Face Toward Player`)
      (`KismetSystemLibrary.Delay` (/ (`PaperFlipbookComponent.GetFlipbookLength` _sprite_2) (`PaperFlipbookComponent.GetPlayRate` _sprite_2)))
      (`SceneComponent.K2_AddRelativeLocation` (`self.Sprite`) (100.0 0.0 0.0) false true)
      (`self.Boss Attack ` (+ (`self.GetActorUpVector`) (* (`self.GetActorForwardVector`) -1.0)) (`self.ComboLaunchIntensity`) (`self.BossDamage`))
      (if (`self.GotHurt`)
        (`self.PositioningTick`)
        (`self.ResetCombo1`)
        (else
          (`self.FindFlipbookBySpritAnimState` "Attack2")
          (`self.Face Toward Player`)
          (`KismetSystemLibrary.Delay` (/ (`PaperFlipbookComponent.GetFlipbookLength` _sprite_3) (`PaperFlipbookComponent.GetPlayRate` _sprite_3)))
          (`self.Boss Attack ` (* (`self.GetActorUpVector`) -1.0) (`self.ComboLaunchIntensity`) (`self.BossDamage`))
          (if (`self.GotHurt`)
            (`self.PositioningTick`)
            (`self.ResetCombo1`)
            (else
              (`self.FindFlipbookBySpritAnimState` "Attack3")
              (`self.Face Toward Player`)
              (`KismetSystemLibrary.Delay` (/ (`PaperFlipbookComponent.GetFlipbookLength` _sprite) (`PaperFlipbookComponent.GetPlayRate` _sprite)))
              (`self.Boss Attack ` (+ (`self.GetActorForwardVector`) (`self.GetActorUpVector`)) (`self.ComboLaunchIntensity`) (`self.BossDamage`))
              (`self.GoForPositioning`)
              (`self.ResetCombo1`))))))))

(event `ResetCombo1`
  (goto _label :!via `Reset`))

(event `ShieldsUp`
  (`/Engine/EditorBlueprintResources/StandardMacros.DoOnce` false :!label _label_2
    (:`Completed`
      (`self.FindFlipbookBySpritAnimState` "Shield")
      (set `self.Shields up` true)
      (`KismetSystemLibrary.Delay` 2.0)
      (`self.GoForPositioning`)
      (goto _label_2 :!via `Reset`))))

(fn `attack`)

(fn `AttackingTick`
  (if (`self.IsDead`)
    _
    (elif (not (`self.IsAttacking`))
      (`self.Combo1`))))

(fn `Boss Attack `
  (params (LaunchDirection :type "Vector Structure") (LaunchIntensity :type "Float (double-precision)") (Damage :type "Float (single-precision)"))
  (locals (PlayerRef :type "/Game/Blueprints/Characters/BP_BigFatHero Object Reference"))
  (bind _playerref (`local.PlayerRef`))
  (`KismetSystemLibrary.PrintString` "Const")
  (bind _outhits (`KismetSystemLibrary.SphereTraceMulti` :`Start` (`SceneComponent.K2_GetComponentLocation` (`self.CapsuleComponent`)) :`End` (`SceneComponent.K2_GetComponentLocation` (`self.HitScanScene`)) :`Radius` (`self.HitScanRadius`) :`TraceChannel` "TraceTypeQuery2" :`TraceColor` (struct :`R` 0.574453 :`B` 1.0 :`A` 1.0)))
  (for _array_element _outhits
    (bind (_bblockinghit _binitialoverlap _time _distance _location _impactpoint _normal _impactnormal _physmat _hitactor) (`GameplayStatics.BreakHitResult` _array_element))
    (if (== _hitactor (`GameplayStatics.GetPlayerPawn` 0))
      (set `local.PlayerRef` (cast `/Game/Blueprints/Characters/BP_BigFatHero` _hitactor :!pure true))
      (break)))
  (`/Engine/EditorBlueprintResources/StandardMacros.IsValid` (`local.PlayerRef`)
    (:`Is Valid`
      (`self.LaunchCharacter` _playerref (* LaunchDirection LaunchIntensity) false false)
      (`self.OnTakeDamage` _playerref Damage self))))

(fn `DefendTick`
  (if (not (`self.IsDead`))
    (`self.ShieldsUp`)))

(fn `Die`)

(fn `Face Toward Player`
  (bind _vec_to_player (`self.GetDirectionToPlayer`))
  (`self.K2_SetActorRotation` (`KismetMathLibrary.MakeRotator` 0.0 0.0 (`KismetMathLibrary.SelectFloat` 180.0 0.0 (> (.yaw (`KismetMathLibrary.MakeRotFromX` _vec_to_player)) 90.0)))))

(fn `FindFlipbookBySpritAnimState`
  (params (`Sprite state` :type "ESpriteAnimState Enum" :default "Idle"))
  (returns (`Out Flipbook` :type "PaperFlipbook Object Reference"))
  (locals (Result :type "PaperFlipbook Object Reference"))
  (bind _result (`local.Result`))
  (set `local.Result` (`.TheFlipBook` (break `AnimFB` (`|GetArrayItem` (`SpriteCharacterDataAsset.SpriteAnimations` (`self.DA_Boss`))))))
  (for _array_element (`SpriteCharacterDataAsset.SpriteAnimations` (`self.DA_Boss`))
    (bind (_animname _theflipbook) (break `AnimFB` _array_element))
    (if (== _animname (`KismetMathLibrary.Conv_ByteToInt` `Sprite state`))
      (set `local.Result` _theflipbook)
      (break)))
  (`PaperFlipbookComponent.SetFlipbook` (`self.Sprite`) _result)
  (return _result))

(fn `GetDirectionToPlayer`
  (returns (`Vec to Player` :type "Vector Structure"))
  (return (- (`self.K2_GetActorLocation` (`GameplayStatics.GetPlayerPawn` 0)) (`self.K2_GetActorLocation`))))

(fn `GoForPositioning`
  (`KismetSystemLibrary.K2_ClearAndInvalidateTimerHandle` (`self.TH_Tick`))
  (bind _returnvalue (`KismetSystemLibrary.K2_SetTimer` null "PositioningTick" 0.01 true))
  (set `self.TH_Tick` _returnvalue))

(fn `InterruptCombo`
  (set `self.GotHurt` true))

(fn `PlayAnim`
  (params (animation :type "/Game/Blueprints/Characters/E_EnemyStates Enum" :default "NewEnumerator0")))

(fn `PositioningTick`
  (bind _sprite (`self.Sprite`))
  (if (not (`self.IsDead`))
    (set `self.Shields up` false)
    (set `self.GotHurt` false)
    (set `self.IsAttacking` false)
    (`self.FindFlipbookBySpritAnimState` "Walk")
    (if (not (`PaperFlipbookComponent.IsPlaying` _sprite))
      (`PaperFlipbookComponent.Play` _sprite))
    (`self.Face Toward Player`)
    (bind _outactors (`GameplayStatics.GetAllActorsOfClass` "/Game/Blueprints/BP_Bullet.BP_Bullet_C"))
    (if (> (`KismetArrayLibrary.Array_Length` _outactors) 0)
      (`KismetSystemLibrary.K2_ClearAndInvalidateTimerHandle` (`self.TH_Tick`))
      (bind _returnvalue (`KismetSystemLibrary.K2_SetTimer` null "DefendTick" 0.01 true))
      (set `self.TH_Tick` _returnvalue)
      (else
        ;[1 1 1] Attack
        (bind (_playerintrackradius _playerinattackradius) (`self.Track Player`))
        (if _playerinattackradius
          (`KismetSystemLibrary.K2_ClearAndInvalidateTimerHandle` (`self.TH_Tick`))
          (bind _returnvalue_2 (`KismetSystemLibrary.K2_SetTimer` null "AttackingTick" 0.01 true))
          (set `self.TH_Tick` _returnvalue_2))))))

(fn `RageMode`
  (`PaperFlipbookComponent.SetPlayRate` (`self.Sprite`) 1.0)
  (set `CharacterMovementComponent.MaxWalkSpeed` 400.0 (`self.CharacterMovement`)))

(fn `Track Player`
  (returns (PlayerInTrackRadius :type Boolean) (PlayerInAttackRadius :type Boolean))
  (bind _returnvalue (- (`self.K2_GetActorLocation` (`GameplayStatics.GetPlayerPawn` 0)) (`self.K2_GetActorLocation`)))
  (bind _returnvalue_2 (`KismetMathLibrary.Normal` _returnvalue))
  (bind _returnvalue_3 (`KismetMathLibrary.VSize` _returnvalue))
  (bind _returnvalue_4 (<= _returnvalue_3 (`self.TrackingRadius`)))
  (if _returnvalue_4
    (`PawnMovementComponent.AddInputVector` (`self.CharacterMovement`) _returnvalue_2 false)
    (set `self.ForwardDir` (.x _returnvalue_2))
    (return _returnvalue_4 (<= _returnvalue_3 (`self.AttackingRadius`)))))

(fn `UpdateAnimation`)

(fn `UserConstructionScript`
  (`PaperFlipbookComponent.SetFlipbook` (`self.Sprite`) (`.TheFlipBook` (break `AnimFB` (`|GetArrayItem` (`SpriteCharacterDataAsset.SpriteAnimations` (`self.DA_Boss`))))))
  (`SceneComponent.K2_SetRelativeLocation` (`self.Sprite`) (`SpriteCharacterDataAsset.SpriteOffset` (`self.DA_Boss`)) false false)
  (`CapsuleComponent.SetCapsuleHalfHeight` (`self.CapsuleComponent`) (`SpriteCharacterDataAsset.CapsuleHalfHeight` (`self.DA_Boss`)) true)
  (`CapsuleComponent.SetCapsuleRadius` (`self.CapsuleComponent`) (`SpriteCharacterDataAsset.CapsuleRadius` (`self.DA_Boss`)) true)
  (`PaperFlipbookComponent.SetPlayRate` (`self.Sprite`) 0.5))