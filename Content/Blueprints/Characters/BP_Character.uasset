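; BP_Character is a character Blueprint that sets up hero input and reports the direction it faces.
; On BeginPlay it adds the IMC_Hero Enhanced Input mapping context for player controller 0.
; GetFaceDirection returns the normalized horizontal vector from the actor's location to BulletSpawnPoint, flattened by using the spawn point's height for both points.
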(event `self.ReceiveBeginPlay`
  (`EnhancedInputSubsystemInterface.AddMappingContext` (pcsubsystem `EnhancedInputLocalPlayerSubsystem` (`GameplayStatics.GetPlayerController` 0)) "/Game/Inputs/IMC_Hero.IMC_Hero" 0 (struct)))

(event `self.ReceiveTick`
  (params (DeltaSeconds :type "Float (single-precision)")))

(fn `GetFaceDirection`
  (returns (FacingDirection :type "Vector Structure"))
  (bind (_returnvalue_x _returnvalue_y) (`KismetMathLibrary.BreakVector` (`self.K2_GetActorLocation`)))
  (bind (_returnvalue_x_2 _returnvalue_y_2 _returnvalue_z) (`KismetMathLibrary.BreakVector` (`SceneComponent.K2_GetComponentLocation` (`self.BulletSpawnPoint`))))
  (bind _output_get (set `self.FacingDirection` (`KismetMathLibrary.Normal` (- (`KismetMathLibrary.MakeVector` _returnvalue_x_2 _returnvalue_y_2 _returnvalue_z) (`KismetMathLibrary.MakeVector` _returnvalue_x _returnvalue_y _returnvalue_z)))))
  (return _output_get))

(fn `UserConstructionScript`)