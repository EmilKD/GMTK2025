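; Side-scrolling 2D player character that runs, jumps, crouches and fires projectiles.
; Enhanced Input drives movement, flipping the sprite and bullet spawn point to face the input direction.
; Shooting spawns BP_Bullet with randomized height, angle and speed, adding the player's velocity to the launch.
; Each tick selects a flipbook from ground state, velocity and the crouch flag, which crouch input sets without calling Crouch.
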(event `self.ReceiveBeginPlay`
  ;[1 1 1] Startup
  (bind _asplayer_controller (cast `PlayerController` (`self.GetController`)))
  (`EnhancedInputSubsystemInterface.AddMappingContext` (pcsubsystem `EnhancedInputLocalPlayerSubsystem` _asplayer_controller) "/Game/Inputs/IMC_Hero.IMC_Hero" 0 (struct)))

(event `EnhancedInput|/Game/Inputs/IA_Jump`
  (params (ActionValue :type "Float (double-precision)") (ElapsedSeconds :type "Float (double-precision)") (TriggeredSeconds :type "Float (double-precision)") (InputAction :type "InputAction Object Reference" :default "/Game/Inputs/IA_Jump.IA_Jump"))
  ;[1 1 1] Movement
  (:`Triggered`
    (`/Engine/EditorBlueprintResources/StandardMacros.DoOnce` false :!label _label
      (:`Completed`
        (`self.Jump`))))
  (:`Completed`
    (goto _label :!via `Reset`)))

(event `EnhancedInput|/Game/Inputs/IA_Move`
  (params (ActionValue :type "Float (double-precision)") (ElapsedSeconds :type "Float (double-precision)") (TriggeredSeconds :type "Float (double-precision)") (InputAction :type "InputAction Object Reference" :default "/Game/Inputs/IA_Move.IA_Move"))
  (bind _bulletspawnpoint (`self.BulletSpawnPoint`))
  ;[1 1 1] Movement
  (:`Triggered`
    (`self.AddMovementInput` (`KismetMathLibrary.Conv_RotatorToVector` (`self.GetControlRotation`)) ActionValue)
    (if (> ActionValue 0.0)
      (`SceneComponent.K2_SetWorldRotation` _bulletspawnpoint (`KismetMathLibrary.MakeRotator` 0.0) false false)
      (`SceneComponent.K2_SetWorldRotation` (`self.Sprite`) (`KismetMathLibrary.MakeRotator` 0.0) false false)
      (set `self.ForwardVec` (1.0 0.0 0.0))
      (else
        (`SceneComponent.K2_SetWorldRotation` _bulletspawnpoint (`KismetMathLibrary.MakeRotator` 0.0 0.0 180.0) false false)
        (`SceneComponent.K2_SetWorldRotation` (`self.Sprite`) (`KismetMathLibrary.MakeRotator` 0.0 0.0 180.0) false false)
        (set `self.ForwardVec` (-1.0 0.0 0.0))))))

(event `self.ReceiveTick`
  (params (DeltaSeconds :type "Float (single-precision)"))
  ;[1 1 1] Anim Update
  (`self.UpdateAnimation`))

(event `EnhancedInput|/Game/Inputs/IA_Crouch`
  (params (ActionValue :type Boolean) (ElapsedSeconds :type "Float (double-precision)") (TriggeredSeconds :type "Float (double-precision)") (InputAction :type "InputAction Object Reference" :default "/Game/Inputs/IA_Crouch.IA_Crouch"))
  ;[1 1 1] Movement
  (:`Triggered`
    (set `self.IsCrouched` true))
  (:`Completed`
    (set `self.IsCrouched` false)))

(event `EnhancedInput|/Game/Inputs/IA_Shoot`
  (params (ActionValue :type "Float (double-precision)") (ElapsedSeconds :type "Float (double-precision)") (TriggeredSeconds :type "Float (double-precision)") (InputAction :type "InputAction Object Reference" :default "/Game/Inputs/IA_Shoot.IA_Shoot"))
  (bind _returnvalue (* (`KismetMathLibrary.RandomFloatInRange` -1.0 1.0) (`self.ThrowAngleRandomization`)))
  ;[1 1 1] Shoot Projectile
  (:`Triggered`
    (bind _returnvalue_2 (`|SpawnActorFromClass` "/Game/Blueprints/BP_Bullet.BP_Bullet_C" (`KismetMathLibrary.MakeTransform` (+ (.location (`SceneComponent.K2_GetComponentToWorld` (`self.BulletSpawnPoint`))) (`KismetMathLibrary.MakeVector` 0.0 0.0 (* (`KismetMathLibrary.RandomFloatInRange` -1.0 1.0) (`self.ThrowLocRandomization`)))) (`KismetMathLibrary.ComposeRotators` (.rotation (`SceneComponent.K2_GetComponentToWorld` (`self.BulletSpawnPoint`))) (`KismetMathLibrary.MakeRotator` 0.0 _returnvalue)) (.scale (`SceneComponent.K2_GetComponentToWorld` (`self.BulletSpawnPoint`)))) "DontSpawnIfColliding" "MultiplyWithRoot" null null))
    (bind _capsulecollision (`/Game/Blueprints/BP_Bullet.CapsuleCollision` _returnvalue_2))
    (`/Engine/EditorBlueprintResources/StandardMacros.IsValid` _capsulecollision
      (:`Is Valid`
        (`PrimitiveComponent.SetPhysicsLinearVelocity` _capsulecollision (+ (`MovementComponent.Velocity` (`self.CharacterMovement`)) (* (`KismetMathLibrary.RotateAngleAxis` (`self.ForwardVec`) _returnvalue (0.0 1.0 0.0)) (+ (`self.ThrowStrength`) (* (`KismetMathLibrary.RandomFloatInRange` -1.0 1.0) (`self.ThrowStrengthRandomization`))))) false "None")))))

(fn `UpdateAnimation`
  (bind _charactermovement (`self.CharacterMovement`))
  (bind _sprite (`self.Sprite`))
  (bind _iscrouched (`self.IsCrouched`))
  (bind _velocity (`MovementComponent.Velocity` _charactermovement))
  (if (`NavMovementComponent.IsMovingOnGround` _charactermovement)
    (if (> (`KismetMathLibrary.VSize` _velocity) 0.0)
      (if _iscrouched
        (`PaperFlipbookComponent.SetFlipbook` _sprite "/Game/statics/Flipbooks/FB_CrouchWalk1.FB_CrouchWalk1")
        (else
          (`PaperFlipbookComponent.SetFlipbook` _sprite "/Game/statics/Flipbooks/FB_Run1.FB_Run1")))
      (elif _iscrouched
        (`PaperFlipbookComponent.SetFlipbook` _sprite "/Game/statics/Flipbooks/FB_CrouchTransition_Flipbook1.FB_CrouchTransition_Flipbook1")
        (`PaperFlipbookComponent.SetFlipbook` _sprite "/Game/statics/Flipbooks/FB_Crouch_Flipbook.FB_Crouch_Flipbook")
        (else
          (`PaperFlipbookComponent.SetFlipbook` _sprite "/Game/statics/Flipbooks/FB_Idle1.FB_Idle1"))))
    (elif (> (.z _velocity) -100.0)
      (`PaperFlipbookComponent.SetFlipbook` _sprite "/Game/statics/Flipbooks/FB_Jump.FB_Jump")
      (else
        (`PaperFlipbookComponent.SetFlipbook` _sprite "/Game/statics/Flipbooks/FB_Fall1.FB_Fall1")))))

(fn `UserConstructionScript`)