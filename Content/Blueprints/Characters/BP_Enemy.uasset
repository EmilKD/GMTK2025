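; Flipbook-animated 2D enemy, set up as Skeleton or Goblin in construction, that chases the player and attacks in melee.
; Tick tracks the player by X/Z distance and drives a state-based animation update.
; Flipbook-length timers hold one-shot animations, then apply attack damage and knockback to the hero inside the overlap sphere.
; Damage triggers hit or death states; death releases attached bullets into physics before destroying the actor.
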(event `self.ReceiveBeginPlay`
  (add `self.OnTakeAnyDamage` (delegate `TakeDamage`)))

(event `TakeDamage` :!signature `self.OnTakeAnyDamage`
  (params (DamagedActor :type "Actor Object Reference") (Damage :type "Float (single-precision)") (DamageType :type "DamageType Object Reference") (InstigatedBy :type "Controller Object Reference") (DamageCauser :type "Actor Object Reference"))
  (bind _returnvalue (- (`self.Health_0`) Damage))
  (`GameplayStatics.PlaySoundAtLocation` "/Game/statics/Sounds/Cues/SC_EnemyBodyHit.SC_EnemyBodyHit" (`self.K2_GetActorLocation`) (struct) 1.0 1.0 0.0 null null null null)
  (if (> _returnvalue 0.0)
    (set `self.Health_0` _returnvalue)
    (set `self.CurrentState` "NewEnumerator3")
    (else
      (set `self.CurrentState` "NewEnumerator4"))))

(event `self.ReceiveTick`
  (params (DeltaSeconds :type "Float (single-precision)"))
  (`|ExecutionSequence`
    (:`then_0`
      (if (`|EnumInequality` (`self.CurrentState`) "NewEnumerator4")
        (bind (_playerintrackradius _playerinattackradius) (`self.Track Player`))
        (set `self.CanTrack` _playerintrackradius)
        (if (and _playerinattackradius (`self.CanAttack`))
          (if (`|EnumInequality` (`self.CurrentState`) "NewEnumerator3")
            (set `self.CurrentState` "NewEnumerator2")
            (set `self.CanAttack` false)
            (`KismetSystemLibrary.K2_SetTimerDelegate` (delegate `CanAttackAgain`) 1.0)))
        (else
          (`MovementComponent.StopMovementImmediately` (`self.CharacterMovement`)))))
    (:`then_1`
      (`self.UpdateAnimation`))))

(event `CanAttackAgain`
  (set `self.CanAttack` true))

(event `self.Sphere.OnComponentBeginOverlap`
  (params (OverlappedComponent :type "PrimitiveComponent Object Reference") (OtherActor :type "Actor Object Reference") (OtherComp :type "PrimitiveComponent Object Reference") (OtherBodyIndex :type Integer) (bFromSweep :type Boolean) (SweepResult :type "HitResult Structure (by ref)"))
  (bind _asbp_big_fat_hero (cast `/Game/Blueprints/Characters/BP_BigFatHero` OtherActor))
  (set `self.PlayerRef` _asbp_big_fat_hero))

(event `self.Sphere.OnComponentEndOverlap`
  (params (OverlappedComponent :type "PrimitiveComponent Object Reference") (OtherActor :type "Actor Object Reference") (OtherComp :type "PrimitiveComponent Object Reference") (OtherBodyIndex :type Integer))
  (set `self.PlayerRef` null))

(fn `attack`
  (bind _playerref (`self.PlayerRef`))
  (`/Engine/EditorBlueprintResources/StandardMacros.IsValid` _playerref
    (:`Is Valid`
      (`self.LaunchCharacter` _playerref (`KismetMathLibrary.MakeVector` (* (`self.ForwardDir`) (`self.AttackStrength`))) false false)
      (`self.OnTakeDamage` _playerref (`self.AttackDamage_0`) self))))

(fn `Die`
  (bind _outactors (`self.GetAttachedActors` true true))
  (if (`KismetArrayLibrary.Array_IsNotEmpty` _outactors)
    (for _array_element _outactors
      (bind _asbp_bullet (cast `/Game/Blueprints/BP_Bullet` _array_element))
      (`self.K2_DetachFromActor` _asbp_bullet "KeepRelative" "KeepRelative" "KeepRelative")
      (`PrimitiveComponent.SetSimulatePhysics` (`/Game/Blueprints/BP_Bullet.CapsuleCollision` _asbp_bullet) true)))
  (`self.K2_DestroyActor`))

(fn `GetDirectionToPlayer`
  (returns (`Vec to Player` :type "Vector Structure"))
  (bind _returnvalue (`GameplayStatics.GetPlayerPawn` 0))
  (bind _returnvalue_2 (`self.K2_GetActorLocation`))
  (bind (_returnvalue_x _returnvalue_y _returnvalue_z) (`KismetMathLibrary.BreakVector` (- (`self.K2_GetActorLocation` _returnvalue) _returnvalue_2)))
  (`/Engine/EditorBlueprintResources/StandardMacros.IsValid` _returnvalue
    (:`Is Valid`
      (return (`KismetMathLibrary.MakeVector` _returnvalue_x 0.0 _returnvalue_z)))
    (:`Is Not Valid`
      (return _returnvalue_2))))

(fn `OnAnimFinishedPlaying`
  (set `self.FinishedPlayingFlipbookAnim` true)
  (switch `/Game/Blueprints/Characters/E_EnemyStates` (`self.CurrentState`)
    (:`NewEnumerator2`
      (`self.attack`)
      (set `self.CurrentState` "NewEnumerator0"))
    (:`NewEnumerator3`
      (set `self.CurrentState` "NewEnumerator0"))
    (:`NewEnumerator4`
      (`KismetSystemLibrary.PrintString` "dead")
      (`self.Die`))))

(fn `PlayAnim`
  (params (animation :type "/Game/Blueprints/Characters/E_EnemyStates Enum" :default "NewEnumerator0"))
  (bind _anims (`self.Anims`))
  (bind _sprite (`self.Sprite`))
  (set `self.FinishedPlayingFlipbookAnim` false)
  (switch `/Game/Blueprints/Characters/E_EnemyStates` animation
    (:`NewEnumerator0`
      (set `self.CurrentFB` (`BlueprintMapLibrary.Map_Find` _anims "idle"))
      (`PaperFlipbookComponent.SetFlipbook` (`self.Sprite`) (`self.CurrentFB`) :!label _label)
      (set `self.FinishedPlayingFlipbookAnim` true))
    (:`NewEnumerator1`
      (set `self.CurrentFB` (`BlueprintMapLibrary.Map_Find` _anims "run"))
      (goto _label))
    (:`NewEnumerator2`
      (set `self.CurrentFB` (`BlueprintMapLibrary.Map_Find` _anims "attack"))
      (`PaperFlipbookComponent.SetFlipbook` _sprite (`self.CurrentFB`) :!label _label_2)
      (`KismetSystemLibrary.K2_SetTimer` null "OnAnimFinishedPlaying" (`PaperFlipbookComponent.GetFlipbookLength` _sprite) :!label _label_3))
    (:`NewEnumerator3`
      (set `self.CurrentFB` (`BlueprintMapLibrary.Map_Find` _anims "takeHit"))
      (goto _label_2))
    (:`NewEnumerator4`
      (bind _output_get (set `self.CurrentFB` (`BlueprintMapLibrary.Map_Find` _anims "die")))
      (`PaperFlipbookComponent.SetFlipbook` (`self.Sprite`) _output_get)
      (goto _label_3))))

(fn `Track Player`
  (returns (PlayerInTrackRadius :type Boolean) (PlayerInAttackRadius :type Boolean))
  (bind _vec_to_player (`self.GetDirectionToPlayer`))
  (bind _returnvalue (`KismetMathLibrary.VSize` _vec_to_player))
  (bind _returnvalue_2 (<= _returnvalue (`self.TrackingRadius`)))
  (if _returnvalue_2
    (bind _returnvalue_3 (`KismetMathLibrary.Normal` _vec_to_player))
    (`PawnMovementComponent.AddInputVector` (`self.CharacterMovement`) _returnvalue_3 false)
    (set `self.ForwardDir` (.x _returnvalue_3))
    (return _returnvalue_2 (<= _returnvalue (`self.AttackingRadius`)))))

(fn `UpdateAnimation`
  (bind _charactermovement (`self.CharacterMovement`))
  (bind _sprite (`self.Sprite`))
  (bind _sphere (`self.Sphere`))
  (if (< (`self.ForwardDir`) 0.0)
    (`SceneComponent.K2_SetRelativeRotation` _sprite (struct :`Yaw` 180.0) false false)
    (`SceneComponent.K2_SetRelativeLocation` _sphere (38.0 0.0 0.0) false false)
    (else
      (`SceneComponent.K2_SetRelativeRotation` :`self` _sprite)
      (`SceneComponent.K2_SetRelativeLocation` _sphere (-38.0 0.0 0.0) false false)))
  (if (`self.FinishedPlayingFlipbookAnim`)
    (switch `/Game/Blueprints/Characters/E_EnemyStates` (`self.CurrentState`)
      (:`NewEnumerator0`
        (if (`NavMovementComponent.IsMovingOnGround` _charactermovement) :!label _label
          (if (> (`KismetMathLibrary.VSize` (`MovementComponent.Velocity` _charactermovement)) 0.0)
            (`self.PlayAnim` "NewEnumerator1")
            (set `self.CurrentState` "NewEnumerator1")
            (else
              (`self.PlayAnim` "NewEnumerator0")
              (set `self.CurrentState` "NewEnumerator0")))))
      (:`NewEnumerator1`
        (goto _label))
      (:`NewEnumerator2`
        (`self.PlayAnim` "NewEnumerator2"))
      (:`NewEnumerator3`
        (`self.PlayAnim` "NewEnumerator3"))
      (:`NewEnumerator4`
        (`self.PlayAnim` "NewEnumerator4")))))

(fn `UserConstructionScript`
  (bind _capsulecomponent (`self.CapsuleComponent`))
  (switch `/Game/Blueprints/Characters/E_EnemyType` (`self.EnemyType`)
    (:`NewEnumerator0`
      (set `self.Anims` (`|MakeMap` "idle" "/Game/statics/Flipbooks/FB_Skeleton_Idle.FB_Skeleton_Idle" "run" "/Game/statics/Flipbooks/FB_Skeleton_Walk.FB_Skeleton_Walk" "attack" "/Game/statics/Flipbooks/FB_Skeleton_Attack.FB_Skeleton_Attack" "takeHit" "/Game/statics/Flipbooks/FB_Skeleton_Take_Hit.FB_Skeleton_Take_Hit" "die" "/Game/statics/Flipbooks/FB_Skeleton_Death.FB_Skeleton_Death" :!type "Name" :!valuetype "PaperFlipbook Object Reference"))
      (`SceneComponent.K2_SetRelativeLocation` (`self.Sprite`) (0.0 0.0 0.0) false false)
      (`CapsuleComponent.SetCapsuleHalfHeight` _capsulecomponent 62.0 true))
    (:`NewEnumerator1`
      (set `self.Anims` (`|MakeMap` "idle" "/Game/statics/Flipbooks/FB_Goblin_Idle.FB_Goblin_Idle" "run" "/Game/statics/Flipbooks/FB_Goblin_Run.FB_Goblin_Run" "attack" "/Game/statics/Flipbooks/FB_Goblin_Attack.FB_Goblin_Attack" "takeHit" "/Game/statics/Flipbooks/FB_Goblin_Take_Hit.FB_Goblin_Take_Hit" "die" "/Game/statics/Flipbooks/FB_Goblin_Death.FB_Goblin_Death" :!type "Name" :!valuetype "PaperFlipbook Object Reference"))
      (`SceneComponent.K2_SetRelativeLocation` (`self.Sprite`) (0.0 0.0 18.0) false false)
      (`CapsuleComponent.SetCapsuleHalfHeight` _capsulecomponent 60.0 true)))
  (set `self.CurrentState` "NewEnumerator0")
  (`PaperFlipbookComponent.SetFlipbook` (`self.Sprite`) (`BlueprintMapLibrary.Map_Find` (`self.Anims`) "idle")))